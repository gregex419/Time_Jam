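; BP_PickupTemplate is a pickup item template that highlights itself and signals when interaction is possible.
; When any Pawn enters its Box, it turns on custom depth rendering for the Item, enables input from player 0 and sets CanInteract on that player's BP_AnimalCharacter.
; Leaving the Box reverses all three.
; The graph holds no pickup or input handling logic itself.
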(event OnComponentBeginOverlap(Box)
  (params (OverlappedComponent :type Primitive%20Component%20Object%20Reference) (OtherActor :type Actor%20Object%20Reference) (OtherComp :type Primitive%20Component%20Object%20Reference) (OtherBodyIndex :type Integer) (bFromSweep :type Boolean) (SweepResult :type Hit%20Result%20Structure%20%28by%20ref%29))
  (Utilities|Casting|CastToPawn OtherActor)
  (Rendering|SetRenderCustomDepth (Variables|Default|GetItem) true)
  (Input|EnableInput (Game|GetPlayerController 0))
  (bind _asbp_animal_character (Utilities|Casting|CastToBP_AnimalCharacter (Game|Player|GetPlayerPawn 0)))
  (Variables|/Game/Blueprints/GameBase/BP_AnimalCharacter.BP_AnimalCharacter_C|SetCanInteract _asbp_animal_character true))

(event OnComponentEndOverlap(Box)
  (params (OverlappedComponent :type Primitive%20Component%20Object%20Reference) (OtherActor :type Actor%20Object%20Reference) (OtherComp :type Primitive%20Component%20Object%20Reference) (OtherBodyIndex :type Integer))
  (Utilities|Casting|CastToPawn OtherActor)
  (Rendering|SetRenderCustomDepth (Variables|Default|GetItem) false)
  (Input|DisableInput (Game|GetPlayerController 0))
  (bind _asbp_animal_character (Utilities|Casting|CastToBP_AnimalCharacter (Game|Player|GetPlayerPawn 0)))
  (Variables|/Game/Blueprints/GameBase/BP_AnimalCharacter.BP_AnimalCharacter_C|SetCanInteract _asbp_animal_character false))

(fn ConstructionScript)