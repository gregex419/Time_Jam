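; BP_Wallet is a wallet pickup that the player's animal character carries in its mouth.
; The Interact input runs a FlipFlop that alternates between attaching it to the ferret mouth socket on the character mesh and detaching it in place.
; Pickup also calls the character's PickupPhoneMessage.
; The graph has no proximity or overlap check before attaching.
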(event EventBeginPlay
  (|CallParentFunction) ; This node is disabled and will not be called.\nDrag off pins to build functionality.
)

(event Input|ActionEvents|InputActionInteract
  (params (Key :type Key%20Structure :default "None"))
  (:Pressed
    (Utilities|FlowControl|FlipFlop
      (:A
        (bind _asbp_animal_character (Utilities|Casting|CastToBP_AnimalCharacter (Game|GetPlayerCharacter 0)))
        (Class|BPPickupInteraction|PickupPhone(Message) _asbp_animal_character) ; Double click to go to this function
        ;[1 0.5 0] Socket Name = Attach Point
        (Transformation|AttachComponentToComponent self (Variables|/Script/Engine.Character|GetMesh _asbp_animal_character) "Ferret_Mouth_Jnt_01Socket" "SnapToTarget" "SnapToTarget" "KeepWorld" true))
      (:B
        (Utilities|Casting|CastToBP_AnimalCharacter (Game|GetPlayerCharacter 0))
        (Transformation|DetachFromActor self "KeepWorld" "KeepWorld" "KeepWorld")))))

(fn ConstructionScript
  (|CallParentFunction))