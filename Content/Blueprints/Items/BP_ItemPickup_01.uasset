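; BP_ItemPickup_01 is an item pickup that the player's BP_AnimalCharacter can take and place back.
; Overlapping InteractionZone sets CanInteract on the character and CanTakePlace on the item, which gates the Take/PlaceItem event.
; A FlipFlop alternates taking and placing, calling TakingItem or PlacingItem and updating HasItem.
; Carrying is faked by swapping visibility between the item's Sphere and the character's own Sphere.
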(event OnComponentBeginOverlap(InteractionZone)
  (params (OverlappedComponent :type Primitive%20Component%20Object%20Reference) (OtherActor :type Actor%20Object%20Reference) (OtherComp :type Primitive%20Component%20Object%20Reference) (OtherBodyIndex :type Integer) (bFromSweep :type Boolean) (SweepResult :type Hit%20Result%20Structure%20%28by%20ref%29))
  ;[1 1 1] Sends data to the Event Dispatcher "Yeller" in the Third Person Character
  (bind _asbp_animal_character (Utilities|Casting|CastToBP_AnimalCharacter OtherActor))
  (Variables|/Game/Blueprints/GameBase/BP_AnimalCharacter.BP_AnimalCharacter_C|SetCanInteract _asbp_animal_character true)
  ;[1 1 1] Can the player take the item?
  (Variables|Default|SetCanTake/Place true))

(event OnComponentEndOverlap(InteractionZone)
  (params (OverlappedComponent :type Primitive%20Component%20Object%20Reference) (OtherActor :type Actor%20Object%20Reference) (OtherComp :type Primitive%20Component%20Object%20Reference) (OtherBodyIndex :type Integer))
  ;[1 1 1] Sends data to the Event Dispatcher "Yeller" in the Third Person Character
  (bind _asbp_animal_character (Utilities|Casting|CastToBP_AnimalCharacter OtherActor))
  (Variables|/Game/Blueprints/GameBase/BP_AnimalCharacter.BP_AnimalCharacter_C|SetCanInteract _asbp_animal_character false)
  ;[1 1 1] Can the player take the item?
  (Variables|Default|SetCanTake/Place false))

(event Custom|Take/Place%20Item
  (bind _sphere (Variables|Default|GetSphere))
  ;[1 1 1] Taking & Placing the item
  (if (Variables|Default|GetCanTake/Place)
    (bind _asbp_animal_character (Utilities|Casting|CastToBP_AnimalCharacter (Game|Player|GetPlayerPawn 0)))
    (Utilities|FlowControl|FlipFlop
      (:A
        (Default|CallTakingItem)
        (Rendering|SetVisibility _sphere false false)
        ;[1 1 1] In BP_AnimalCharacter
        (Rendering|SetVisibility (Variables|/Game/Blueprints/GameBase/BP_AnimalCharacter.BP_AnimalCharacter_C|GetSphere _asbp_animal_character) true false)
        (Variables|/Game/Blueprints/GameBase/BP_AnimalCharacter.BP_AnimalCharacter_C|SetHasItem _asbp_animal_character true))
      (:B
        (Default|CallPlacingItem)
        (Rendering|SetVisibility _sphere true false)
        (Rendering|SetVisibility (Variables|/Game/Blueprints/GameBase/BP_AnimalCharacter.BP_AnimalCharacter_C|GetSphere _asbp_animal_character) false false)
        (Variables|/Game/Blueprints/GameBase/BP_AnimalCharacter.BP_AnimalCharacter_C|SetHasItem _asbp_animal_character false)))))

(fn ConstructionScript)