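; BP_EnemyAICharacter is an enemy AI character that patrols four target points and chases the player when it sees a BP_AnimalCharacter holding an item.
; PawnSensing triggers either the chase, turning its spotlight red, or random roaming with a white light when no item is held.
; Patrol, roam and chase are AIMoveTo loops that re-run on success after a delay; catching the player prints a tag message.
; An AIState switch exists but is never executed.
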(event OnSeePawn(PawnSensing)
  (params (Pawn :type Pawn%20Object%20Reference))
  (bind _spotlight (Variables|Default|GetSpotLight))
  ;[1 1 1] If you have an object, and are seen, then you will be chased
  (bind _asbp_animal_character (Utilities|Casting|CastToBP_AnimalCharacter Pawn))
  (if (Variables|/Game/Blueprints/GameBase/BP_AnimalCharacter.BP_AnimalCharacter_C|GetHasItem _asbp_animal_character)
    (CallFunction|ChasePlayer)
    (Rendering|Components|Light|SetLightColor _spotlight "(R=1.000000,G=0.000000,B=0.000000,A=1.000000)" true)
    (else
      (CallFunction|RoamAround)
      (Rendering|Components|Light|SetLightColor _spotlight "(R=1.000000,G=1.000000,B=1.000000,A=1.000000)" true))))

(event Custom|Roam%20Around
  ;[1 1 1] Basic Roaming Setup
  (AI|AIMoveTo self (.RandomLocation (Class|NavigationSystemV1|GetRandomPointinNavigableRadius (Transformation|GetActorLocation) 5e+02 0 0)) 0 5.0 false
    (:OnSuccess
      (Utilities|FlowControl|Delay 1.0)
      (CallFunction|RoamAround))))

(event Custom|Chase%20Player
  ;[1 1 1] Basic Player Chase
  (AI|AIMoveTo self "0, 0, 0" (Game|GetPlayerCharacter 0) 5.0 false
    (:OnSuccess
      ;;[1 0.5 0] Event for when you're caught
      (Development|PrintString "Tag! You're it!")
      (Utilities|FlowControl|Delay 1.0)
      (CallFunction|ChasePlayer))))

(event Custom|Patrol
  (bind _self self)
  ;[1 1 1] Basic Patrol
  (AI|AIMoveTo _self "0, 0, 0" (Variables|Default|GetTargetPoint1) 5.0 false
    (:OnSuccess
      (Utilities|FlowControl|Delay 1.0)
      (AI|AIMoveTo _self "0,0.000000, 0" (Variables|Default|GetTargetPoint2) 5.0 false
        (:OnSuccess
          (Utilities|FlowControl|Delay 1.0)
          (AI|AIMoveTo _self "0, 0, 0" (Variables|Default|GetTargetPoint3) 5.0 false
            (:OnSuccess
              (Utilities|FlowControl|Delay 1.0)
              (AI|AIMoveTo _self "0,0.000000, 0" (Variables|Default|GetTargetPoint4) 5.0 false
                (:OnSuccess
                  (Utilities|FlowControl|Delay 1.0)
                  (CallFunction|Patrol))))))))))

(event EventBeginPlay
  ;[1 1 1] Debugging
  (CallFunction|Patrol))

(fn ConstructionScript)