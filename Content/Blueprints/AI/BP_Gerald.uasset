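; BP_Gerald is an AI pawn that patrols, roams and chases the player when it sees an animal character carrying an item.
; After a head-start delay, it chains AIMoveTo calls through three patrol points, using lead-in points for facing, then roams randomly before patrolling again.
; AI perception starts the chase or resumes patrol; losing sight of an item carrier triggers roaming, then delayed patrol.
; An AIState switch offers manual behavior selection but is not called here.
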(event OnTargetPerceptionUpdated(AIPerception)
  (params (Actor :type Actor%20Object%20Reference) (Stimulus :type AI%20Stimulus%20Structure))
  ;[1 1 1] What happens when the player is seen (Figure out entering and exiting the pawn sensing... Specifically Exiting)
  (bind _asbp_animal_character (Utilities|Casting|CastToBP_AnimalCharacter Actor))
  ;;[1 1 1] True = Player is seen
  ;; Fales = Lost Sight of Player
  (if (.bSuccessfullySensed (Utilities|Struct|BreakAIStimulus Stimulus))
    (Variables|/Game/Blueprints/GameBase/BP_AnimalCharacter.BP_AnimalCharacter_C|SetIsSeen _asbp_animal_character true)
    (if (Variables|/Game/Blueprints/GameBase/BP_AnimalCharacter.BP_AnimalCharacter_C|GetHasItem _asbp_animal_character)
      (CallFunction|ChasePlayer)
      (else
        (CallFunction|Patrol :!label _label)))
    (elif (Variables|/Game/Blueprints/GameBase/BP_AnimalCharacter.BP_AnimalCharacter_C|GetHasItem _asbp_animal_character)
      (Utilities|FlowControl|Sequence
        (:then_0
          _)
        (:then_1
          _)
        (:then_2
          _)
        (:then_3
          (Utilities|FlowControl|Delay 5.0)
          (goto _label)))
      (CallFunction|RoamAround))))

(event Custom|Roam%20Around
  ;[1 1 1] AI Behavior Setup
  ;;[0 1 0] Basic Roaming Setup
  (AI|AIMoveTo self (.RandomLocation (Class|NavigationSystemV1|GetRandomPointinNavigableRadius (Transformation|GetActorLocation) 5e+02 0 0)) 0 0.01 false
    (:OnSuccess
      (Utilities|FlowControl|Delay 1.0) ; Wait time between points
      (Variables|Default|SetRoamCounter (- (Variables|Default|GetRoamCounter) 1))
      (if (== (Variables|Default|GetRoamCounter) 0)
        (CallFunction|Patrol)
        (else
          (CallFunction|RoamAround))))))

(event Custom|Chase%20Player
  ;[1 1 1] AI Behavior Setup
  ;;[1 0 0] Basic Player Chase
  (Development|PrintString "Chasing")
  (AI|AIMoveTo self "0, 0, 0" (Game|GetPlayerCharacter 0) 0.01 false
    (:OnSuccess
      ;;;[1 0.5 0] Event for when you're caught
      (Development|PrintString "Tag! You're it!")
      (Utilities|FlowControl|Delay 1.0)
      (CallFunction|ChasePlayer))))

(event Custom|Head%20Start
  ;[1 1 1] Checks to see if head start is complete
  ;;[1 0.5 0] Head Start Delay
  (Utilities|FlowControl|Delay 5.0)
  (CallFunction|Patrol))

(event Custom|AI%20Switches
  ;[1 1 1] Manual Control System (Switches)
  (switch Utilities|FlowControl|Switch|SwitchonEnum_AI_State (Variables|Default|GetAIState)
    (:NewEnumerator1
      (CallFunction|RoamAround))
    (:NewEnumerator2
      (CallFunction|ChasePlayer))
    (:NewEnumerator3
      (CallFunction|Patrol))))

(event Custom|Patrol
  ;[1 1 1] AI Behavior Setup
  ;;[0 0 1] AI Patrol
  ;;;[1 1 1] Event Patrol
  ;;;[1 1 1] This sends the AI to a point right before the main point. Use the first set of points to have the character facing the right direction when they get to the inportant target point.
  ;;;;[1 1 1] Moves the AI to its destination
  (AI|AIMoveTo self "0, 0, 0" (Utilities|Array|Get(acopy) (Variables|Default|GetPatrolPoints) (Variables|Default|GetPatrolPointsIndex)) 0.1 false ; Acceptance Radius = How Close To Target
    (:OnSuccess
      ;;;;[1 1 1] Returns if you have reached the end of the patrol points or not...
      (if (>= (Variables|Default|GetPatrolPointsIndex) (- (Utilities|Array|Length (Variables|Default|GetPatrolPoints)) 1))
        ;;;;[1 1 1] Resets the patrol points to 0
        (Variables|Default|SetPatrolPointsIndex 0)
        (else
          ;;;;[1 1 1] Incriments to the next patrol point
          (Math|Integer|IncrementInt (Variables|Default|GetPatrolPointsIndex)
            (:%20%20
              _))))
      ;;;[1 1 1] This sends the AI to a point right before the main point. Use the first set of points to have the character facing the right direction when they get to the inportant target point.
      ;;;;[1 1 1] Moves the AI to its destination
      (AI|AIMoveTo self "0, 0, 0" (Utilities|Array|Get(acopy) (Variables|Default|GetPatrolPoints) (Variables|Default|GetPatrolPointsIndex)) 0.1 false ; Acceptance Radius = How Close To Target
        (:OnSuccess
          ;;;;[1 1 1] Returns if you have reached the end of the patrol points or not...
          (if (>= (Variables|Default|GetPatrolPointsIndex) (- (Utilities|Array|Length (Variables|Default|GetPatrolPoints)) 1))
            ;;;;[1 1 1] Resets the patrol points to 0
            (Variables|Default|SetPatrolPointsIndex 0)
            (else
              ;;;;[1 1 1] Incriments to the next patrol point
              (Math|Integer|IncrementInt (Variables|Default|GetPatrolPointsIndex)
                (:%20%20
                  _))))
          ;;;[1 1 1] This is the actual point you want to go to.
          ;;;;[1 1 1] Moves the AI to its destination
          (AI|AIMoveTo self "0, 0, 0" (Utilities|Array|Get(acopy) (Variables|Default|GetPatrolPoints) (Variables|Default|GetPatrolPointsIndex)) 0.1 false ; Acceptance Radius = How Close To Target
            (:OnSuccess
              ;;;;[1 1 1] Returns if you have reached the end of the patrol points or not...
              (if (>= (Variables|Default|GetPatrolPointsIndex) (- (Utilities|Array|Length (Variables|Default|GetPatrolPoints)) 1))
                ;;;;[1 1 1] Resets the patrol points to 0
                (Variables|Default|SetPatrolPointsIndex 0)
                (else
                  ;;;;[1 1 1] Incriments to the next patrol point
                  (Math|Integer|IncrementInt (Variables|Default|GetPatrolPointsIndex)
                    (:%20%20
                      _))))
              ;;;;[1 0.5 0] Time Between Targets
              (Utilities|FlowControl|Delay 1.0)
              ;;;[1 1 1] Roam Setup
              (Variables|Default|SetRoamCounter (Math|Random|RandomIntegerinRange 3 8))
              (CallFunction|RoamAround))))))))

(event EventBeginPlay
  (CallFunction|HeadStart))

(event EventTick
  (params (DeltaSeconds :type Float%20%28single-precision%29)))

(fn ConstructionScript)