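; Owner AI pawn that roams, patrols or chases the player's animal character, using AIMoveTo behaviors that re-trigger themselves on success.
; An AIState switch picks the behavior: random navmesh roaming, looping through PatrolPoints, or chasing with a debug "tag" message on arrival.
; Pawn sensing flags the player as seen, then turns the spotlight red and chases if they hold an item, otherwise green and patrols.
; Losing sight is not handled.
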(event OnSeePawn(PawnSensing)
  (params (Pawn :type Pawn%20Object%20Reference))
  (bind _spotlight (Variables|Default|GetSpotLight))
  ;[1 1 1] What happens when the player is seen (Figure out entering and exiting the pawn sensing... Specifically Exiting)
  (bind _asbp_animal_character (Utilities|Casting|CastToBP_AnimalCharacter (Game|Player|GetPlayerPawn 0)))
  (Variables|/Game/Blueprints/GameBase/BP_AnimalCharacter.BP_AnimalCharacter_C|SetIsSeen _asbp_animal_character true)
  (if (Variables|/Game/Blueprints/GameBase/BP_AnimalCharacter.BP_AnimalCharacter_C|GetHasItem _asbp_animal_character)
    (Rendering|Components|Light|SetLightColor _spotlight "(R=1.000000,G=0.000000,B=0.000000,A=1.000000)" true)
    (CallFunction|ChasePlayer)
    (else
      (Rendering|Components|Light|SetLightColor _spotlight "(R=0.000000,G=1.000000,B=0.000000,A=1.000000)" true)
      ;;[1 0.5 0] Replace with advanced Patrol/Roam
      (CallFunction|Patrol))))

(event Custom|Roam%20Around
  ;[1 1 1] Basic Roaming Setup
  (Development|PrintString "Roaming")
  (AI|AIMoveTo self (.RandomLocation (Class|NavigationSystemV1|GetRandomPointinNavigableRadius (Transformation|GetActorLocation) 1e+03 0 0)) 0 1.0 false
    (:OnSuccess
      (Utilities|FlowControl|Delay 0.5) ; Wait time between points
      (CallFunction|RoamAround))))

(event Custom|Chase%20Player
  ;[1 1 1] Basic Player Chase
  (Development|PrintString "Chasing")
  (AI|AIMoveTo self "0, 0, 0" (Game|GetPlayerCharacter 0) 5.0 false
    (:OnSuccess
      ;;[1 0.5 0] Event for when you're caught
      (Development|PrintString "Tag! You're it!")
      (Utilities|FlowControl|Delay 1.0)
      (CallFunction|ChasePlayer))))

(event Custom|Patrol
  ;[1 1 1] Patrol
  (Development|PrintString "Patroling")
  (AI|AIMoveTo self "0, 0, 0" (Utilities|Array|Get(acopy) (Variables|Default|GetPatrolPoints) (Variables|Default|GetPatrolPointIndex)) 1.0 false ; Acceptance Radius = How Close To Target
    (:OnSuccess
      (Utilities|FlowControl|Delay 2.0) ; Time Between Targets
      (if (>= (Variables|Default|GetPatrolPointIndex) (- (Utilities|Array|Length (Variables|Default|GetPatrolPoints)) 1))
        (Variables|Default|SetPatrolPointIndex 0)
        (else
          (Math|Integer|IncrementInt (Variables|Default|GetPatrolPointIndex)
            (:%20%20
              _))))
      (Development|PrintString "Target." true true "(R=1.000000,G=0.500000,B=1.000000,A=1.000000)" 1.0)
      (CallFunction|Patrol))))

(event Custom|AI%20Event%20Sequence
  ;[1 1 1] AI State Event Sequence
  (switch Utilities|FlowControl|Switch|SwitchonEnum_AI_State (Variables|Default|GetAIState)
    (:NewEnumerator0
      (CallFunction|RoamAround :!label _label))
    (:NewEnumerator1
      (goto _label))
    (:NewEnumerator2
      (CallFunction|ChasePlayer))
    (:NewEnumerator3
      (CallFunction|Patrol))))

(event EventBeginPlay
  (CallFunction|AIEventSequence))

(fn ConstructionScript)